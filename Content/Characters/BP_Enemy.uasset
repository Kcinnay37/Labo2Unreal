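; BP_Enemy is an enemy character Blueprint that reacts to the player and displays a health bar.
; Overlaps on its Perception component cast to MyPlayer and call OnPerception or OnPerceptionEnd, which are defined outside this graph.
; Events show or hide the Slider widget component, push the health percentage into its WPB_SliderEnemy progress bar, and rotate it toward the player camera as a billboard.
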(event OnComponentBeginOverlap(Perception)
  (params (OverlappedComponent :type Primitive%20Component%20Object%20Reference) (OtherActor :type Actor%20Object%20Reference) (OtherComp :type Primitive%20Component%20Object%20Reference) (OtherBodyIndex :type Integer) (bFromSweep :type Boolean) (SweepResult :type Hit%20Result%20Structure%20%28by%20ref%29))
  (bind _asmy_player (Utilities|Casting|CastToMyPlayer OtherActor))
  (Class|MyEnemy|OnPerception _asmy_player))

(event OnComponentEndOverlap(Perception)
  (params (OverlappedComponent :type Primitive%20Component%20Object%20Reference) (OtherActor :type Actor%20Object%20Reference) (OtherComp :type Primitive%20Component%20Object%20Reference) (OtherBodyIndex :type Integer))
  (Utilities|Casting|CastToMyPlayer OtherActor)
  (Class|MyEnemy|OnPerceptionEnd))

(event EventShowSlider
  (Rendering|SetVisibility (Variables|Default|GetSlider) true false))

(event EventUnShowSlider
  (Rendering|SetVisibility (Variables|Default|GetSlider) false false))

(event EventRotateSlider
  (bind _slider (Variables|Default|GetSlider))
  (Transformation|SetWorldRotation _slider (Math|Rotator|FindLookatRotation (Transformation|GetWorldLocation _slider) (Camera|GetCameraLocation (Game|GetPlayerCameraManager 0))) false false))

(event EventOnHealthChanged
  (bind _aswpb_slider_enemy (Utilities|Casting|CastToWPB_SliderEnemy (UserInterface|GetWidget (Variables|Default|GetSlider))))
  (bind _returnvalue (Class|Avatar|GetPercentHealth))
  (Progress|SetPercent (Variables|/Game/Characters/WPB_SliderEnemy.WPB_SliderEnemy_C|GetProgressBar_0 _aswpb_slider_enemy) _returnvalue))

(fn ConstructionScript)