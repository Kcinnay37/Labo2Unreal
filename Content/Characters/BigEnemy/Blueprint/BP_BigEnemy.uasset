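; BP_BigEnemy is a large enemy character that drops a quest item when it dies.
; Its Dead event spawns BP_QuestItem at the DropLocation component and plays a zombie creature breath sound at the actor's position.
; The same event makes the capsule ignore WorldDynamic and Camera channels and the mesh ignore WorldDynamic.
; The construction script only calls its parent, and the graphs hold no other behavior.
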(event EventDead
  (Game|SpawnActorfromClass "/Game/Blueprint/BP_QuestItem.BP_QuestItem_C" (Math|Conversions|ToTransform(Vector) (Transformation|GetWorldLocation (Variables|Default|GetDropLocation))) "Undefined" 0 0)
  (Collision|SetCollisionResponsetoChannel (Variables|Default|GetCapsuleComponent) "ECC_WorldDynamic" "ECR_Ignore")
  (Collision|SetCollisionResponsetoChannel (Variables|Default|GetCapsuleComponent) "ECC_Camera" "ECR_Ignore")
  (Collision|SetCollisionResponsetoChannel (Variables|Character|GetMesh) "ECC_WorldDynamic" "ECR_Ignore")
  (Audio|PlaySoundatLocation "/Game/Audio/Died/ES_Zombie_Creature_Breath_10_-_SFX_Producer.ES_Zombie_Creature_Breath_10_-_SFX_Producer" (Transformation|GetActorLocation) "0, 0, 0" 1.0 1.0 0.0 0 0 0))

(fn ConstructionScript
  (|CallParentFunction))