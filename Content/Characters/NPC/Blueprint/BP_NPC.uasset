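; NPC character that gives the player quest dialogue and triggers the game win once they have the required resource.
; Entering its TalkPerception overlap shows a push-to-talk widget and registers a delegate on the player's TheBossController; leaving removes both, plus any dialogue.
; Talking swaps the prompt for a dialogue widget with quest or win text, calling OnWinGame on the game mode for the latter.
; ABP_NPC's IsTalking flag drives the talk animation.
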(event OnComponentBeginOverlap(TalkPerception)
  (params (OverlappedComponent :type Primitive%20Component%20Object%20Reference) (OtherActor :type Actor%20Object%20Reference) (OtherComp :type Primitive%20Component%20Object%20Reference) (OtherBodyIndex :type Integer) (bFromSweep :type Boolean) (SweepResult :type Hit%20Result%20Structure%20%28by%20ref%29))
  (CallFunction|OnTalkPerception OtherActor))

(event OnComponentEndOverlap(TalkPerception)
  (params (OverlappedComponent :type Primitive%20Component%20Object%20Reference) (OtherActor :type Actor%20Object%20Reference) (OtherComp :type Primitive%20Component%20Object%20Reference) (OtherBodyIndex :type Integer))
  (CallFunction|EndTalkPerception OtherActor))

(event EventTalktoNPC
  (CallFunction|OnTalk))

(fn ConstructionScript)

(fn OnTalkPerception
  (params (Other :type Actor%20Object%20Reference%20%28by%20ref%29))
  (bind _asmy_player (Utilities|Casting|CastToMyPlayer Other))
  (bind _asthe_boss_controller (Utilities|Casting|CastToTheBossController (Pawn|GetController _asmy_player)))
  (bind _output_get (Variables|Default|Setthe%20Boss%20Controller _asthe_boss_controller))
  (Class|NPC|AddDelegatetoPlayer _output_get)
  (Utilities|IsValid (Variables|Default|GetPushToTalkWidget)
    (:Is%20Valid
      _)
    (:Is%20Not%20Valid
      (bind _returnvalue (UserInterface|CreateWidget "/Game/Characters/NPC/WBP_NPCPushToTalk.WBP_NPCPushToTalk_C" _output_get))
      (Variables|Default|SetPushToTalkWidget _returnvalue)))
  (UserInterface|Viewport|AddtoViewport (Variables|Default|GetPushToTalkWidget) 0))

(fn EndTalkPerception
  (params (Other :type Actor%20Object%20Reference%20%28by%20ref%29))
  (bind _asmy_player (Utilities|Casting|CastToMyPlayer Other))
  (CallFunction|SetTalkAnim false)
  (bind _asthe_boss_controller (Utilities|Casting|CastToTheBossController (Pawn|GetController _asmy_player)))
  (Class|NPC|RemoveDelegatetoPlayer _asthe_boss_controller)
  (Utilities|FlowControl|Sequence
    (:then_0
      (Utilities|IsValid (Variables|Default|GetPushToTalkWidget)
        (:Is%20Valid
          (Widget|RemovefromParent (Variables|Default|GetPushToTalkWidget)))))
    (:then_1
      (Utilities|IsValid (Variables|Default|GetNPCDialgogue)
        (:Is%20Valid
          (Widget|RemovefromParent (Variables|Default|GetNPCDialgogue)))))))

(fn OnTalk
  (CallFunction|SetTalkAnim true)
  (Class|NPC|RemoveDelegatetoPlayer (Variables|Default|Getthe%20Boss%20Controller))
  (Widget|RemovefromParent (Variables|Default|GetPushToTalkWidget))
  (Utilities|IsValid (Variables|Default|GetNPCDialgogue)
    (:Is%20Valid
      _)
    (:Is%20Not%20Valid
      (bind _returnvalue (UserInterface|CreateWidget "/Game/Characters/NPC/WBP_NPCDialogue.WBP_NPCDialogue_C" (Variables|Default|Getthe%20Boss%20Controller)))
      (Variables|Default|SetNPCDialgogue _returnvalue)))
  (UserInterface|Viewport|AddtoViewport (Variables|Default|GetNPCDialgogue) 0)
  (bind _returnvalue_2 (Class|NPC|GetPlayerHaveResource (Variables|Default|Getthe%20Boss%20Controller)))
  (if _returnvalue_2
    (Rendering|Components|TextRender|SetText (Variables|/Game/Characters/NPC/WBP_NPCDialogue.WBP_NPCDialogue_C|GetMultiLineEditableTextBox_0 (Variables|Default|GetNPCDialgogue)) (Utilities|Text|ToText(String) (Variables|Default|GetdialogueWin)))
    (bind _aslabo_2unreal_game_mode_base (Utilities|Casting|CastToLabo2UnrealGameModeBase (Game|GetGameMode)))
    (Class|Labo2UnrealGameModeBase|OnWinGame _aslabo_2unreal_game_mode_base)
    (else
      (Rendering|Components|TextRender|SetText (Variables|/Game/Characters/NPC/WBP_NPCDialogue.WBP_NPCDialogue_C|GetMultiLineEditableTextBox_0 (Variables|Default|GetNPCDialgogue)) (Utilities|Text|ToText(String) (Variables|Default|GetdialogueQuest))))))

(fn SetTalkAnim
  (params (Talk :type Boolean))
  (bind _asabp_npc (Utilities|Casting|CastToABP_NPC (Components|SkeletalMesh|GetAnimInstance (Variables|Character|GetMesh))))
  (Variables|/Game/Characters/NPC/Anim/ABP_NPC.ABP_NPC_C|SetIsTalking _asabp_npc Talk))