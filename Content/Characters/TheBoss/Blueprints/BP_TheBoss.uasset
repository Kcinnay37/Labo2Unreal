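; BP_TheBoss is a character Blueprint that manages the player's HUD for the boss character.
; On BeginPlay it creates health bar and inventory widgets for the owning player controller, adds them to the viewport and sets the portrait texture.
; Health and equipped-item change events then push the health percentage, item count and item icon straight into those widgets' elements.
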(event EventBeginPlay
  (Utilities|FlowControl|Sequence
    (:then_0
      ;[1 1 1] Ajout des widget
      (bind _asplayer_controller (Utilities|Casting|CastToPlayerController (Pawn|GetController)))
      (bind _returnvalue (UserInterface|CreateWidget "/Game/Characters/TheBoss/WBP_HealthBar.WBP_HealthBar_C" _asplayer_controller))
      (bind _output_get (Variables|Default|SetHealthBarWidget _returnvalue))
      (UserInterface|Viewport|AddtoViewport _output_get 0)
      (bind _returnvalue_2 (UserInterface|CreateWidget "/Game/Characters/TheBoss/WBP_Inventory.WBP_Inventory_C" _asplayer_controller))
      (bind _output_get_2 (Variables|Default|SetInventoryWidget _returnvalue_2))
      (UserInterface|Viewport|AddtoViewport _output_get_2 0))
    (:then_1
      ;[1 1 1] Ajout des texture
      (bind _returnvalue_3 (Class|Avatar|GetPortrait))
      (Appearance|SetBrushfromTexture (Variables|/Game/Characters/TheBoss/WBP_HealthBar.WBP_HealthBar_C|GetPortrait (Variables|Default|GetHealthBarWidget)) _returnvalue_3 false))))

(event EventOnNbItemEquipChanged
  (params (currNb :type Integer) (currTexture :type Texture%202D%20Object%20Reference))
  (Rendering|Components|TextRender|SetText (Variables|/Game/Characters/TheBoss/WBP_Inventory.WBP_Inventory_C|GetNumber (Variables|Default|GetInventoryWidget)) (Utilities|Text|ToText(Integer) currNb))
  (Appearance|SetBrushfromTexture (Variables|/Game/Characters/TheBoss/WBP_Inventory.WBP_Inventory_C|GetItemImage (Variables|Default|GetInventoryWidget)) currTexture false))

(event EventOnHealthChanged
  ;[1 1 1] Change la vie dans la barre de vie
  (bind _returnvalue (Class|Avatar|GetPercentHealth))
  (Progress|SetPercent (Variables|/Game/Characters/TheBoss/WBP_HealthBar.WBP_HealthBar_C|GetTheBar (Variables|Default|GetHealthBarWidget)) _returnvalue))

(fn ConstructionScript)